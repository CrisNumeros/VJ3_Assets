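; Health pickup actor that heals the player on contact.
; Its model rotates a fixed yaw step every tick.
; When the collision component overlaps a BP_Player, it adds health through the player's Interfaz AddVida call with shield off, plays a healing sound at its location and destroys itself.
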(event `self.ReceiveTick`
  (params (DeltaSeconds :type "Float (single-precision)"))
  (`SceneComponent.K2_AddWorldRotation` (`self.Modelo`) (struct :`Yaw` 1.0) false false))

(event `self.Collision.OnComponentBeginOverlap`
  (params (OverlappedComponent :type "PrimitiveComponent Object Reference") (OtherActor :type "Actor Object Reference") (OtherComp :type "PrimitiveComponent Object Reference") (OtherBodyIndex :type Integer) (bFromSweep :type Boolean) (SweepResult :type "HitResult Structure (by ref)"))
  (bind _asbp_player (cast `/Game/ThirdPersonBP/Blueprints/BP_Player` OtherActor))
  (`/Game/_objetos/Interfaces/Interfaz_Player.AddVida` (`/Game/ThirdPersonBP/Blueprints/BP_Player.Interfaz` _asbp_player) 15.0 false)
  (`GameplayStatics.PlaySoundAtLocation` "/Game/_objetos/Sonidos/s_Curacion.s_Curacion" (`SceneComponent.K2_GetComponentLocation` (`self.Modelo`)) (struct) 1.0 1.0 0.0 null null null)
  (`self.K2_DestroyActor` self))

(fn `UserConstructionScript`)