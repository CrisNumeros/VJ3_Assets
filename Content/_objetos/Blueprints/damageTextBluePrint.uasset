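; Floating damage number actor that displays a damage value as animated text.
; PlayDamageText sets and shows the text, then plays the PlayAnimation timeline.
; The timeline drives height above the spawn point, roll and scale, using a random roll range and per-update Y drift picked at BeginPlay to vary each number.
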(event `self.ReceiveBeginPlay`
  (set `self.AntPosition` (`self.K2_GetActorLocation` self))
  (set `self.AntRotation` (`self.K2_GetActorRotation` self))
  (set `self.XRotation` (`KismetMathLibrary.RandomFloatInRange` -40.0 40.0))
  (set `self.YRandom` (`KismetMathLibrary.RandomFloatInRange` -5.0 5.0)))

(fn `PlayDamageText`
  (params (damage :type "Float (double-precision)"))
  (`TextRenderComponent.K2_SetText` (`self.texto`) (`KismetTextLibrary.Conv_DoubleToText` damage "HalfToEven"))
  (`TimelineComponent.Play` (`self.PlayAnimation`))
  (`SceneComponent.SetVisibility` (`self.texto`) true false))

(fn `UserConstructionScript`)