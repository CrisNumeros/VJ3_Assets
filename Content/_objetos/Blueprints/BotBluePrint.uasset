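; BotBluePrint is an early bot Blueprint with a hand-rolled timer and a Mira overlap component.
; Each Tick accumulates delta time into a counter that resets after passing ten seconds, then runs MiraFunction.
; MiraFunction uses GetTime to check the counter against a two-second threshold, but the branch does nothing yet.
; An overlap on Mira only prints a debug greeting.
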(event `self.ReceiveTick`
  (params (DeltaSeconds :type "Float (single-precision)"))
  (`self.DeltaTimeFunction` DeltaSeconds)
  (`self.MiraFunction`))

(event `self.Mira.OnComponentBeginOverlap`
  (params (OverlappedComponent :type "PrimitiveComponent Object Reference") (OtherActor :type "Actor Object Reference") (OtherComp :type "PrimitiveComponent Object Reference") (OtherBodyIndex :type Integer) (bFromSweep :type Boolean) (SweepResult :type "HitResult Structure (by ref)"))
  (`KismetSystemLibrary.PrintString` "Hello"))

(fn `DeltaTimeFunction`
  (params (deltaTime :type "Float (double-precision)"))
  (bind _output_get (set `self._deltaTimeCount` (+ deltaTime (`self._deltaTimeCount`))))
  (if (> _output_get 10.0)
    (set `self._deltaTimeCount` 0.0)))

(fn `GetTime`
  (params (time :type "Float (double-precision)"))
  (returns (isTime :type Boolean))
  (return (< time (`self._deltaTimeCount`))))

(fn `MiraFunction`
  (bind _istime (`self.GetTime` 2.0))
  (if _istime
    _))

(fn `UserConstructionScript`)